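; Parent Blueprint for an addendum namecard actor that displays a person's name as 3D text on a card mesh.
; OnInteraction, gated by ShowNamecard, toggles visibility from Hidden, then reapplies PersonName and the mesh matching NamecardType.
; The construction script previews text and mesh with validity checks, but its Horizontal mesh assignment is unconnected.
; GetLevelName is an empty stub and IsHovering always returns false.
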(event EventBeginPlay)

(event Collision|EventActorBeginOverlap
  (params (OtherActor :type Actor%20Object%20Reference)))

(event EventTick
  (params (DeltaSeconds :type Float%20%28single-precision%29)))

(event EventOnInteraction
  (bind _namecard (Variables|Default|GetNamecard))
  (if (Variables|InteractionControls|GetbShowNamecard)
    (if (Variables|Rendering|GetbHidden)
      (Rendering|SetActorHiddenInGame false)
      (else
        (Rendering|SetActorHiddenInGame true)))
    (Utilities|FlowControl|Sequence
      (:then_0
        (Variables|/Script/Text3D.Text3DComponent|SetText (Variables|Default|GetText3D) (Variables|InteractionControls|GetPersonName)))
      (:then_1
        (switch Utilities|FlowControl|Switch|SwitchonE_NamecardType (Variables|InteractionControls|GetNamecardType)
          (:NewEnumerator0
            (Components|StaticMesh|SetStaticMesh _namecard "/Game/HungryGaussians/Assets/Models/Namecard/RoundedNamecard.RoundedNamecard"))
          (:NewEnumerator1
            (Components|StaticMesh|SetStaticMesh _namecard "/Game/HungryGaussians/Assets/Models/Namecard/VerticalNamecard.VerticalNamecard"))
          (:NewEnumerator2
            (Components|StaticMesh|SetStaticMesh _namecard "/Game/HungryGaussians/Assets/Models/Namecard/HorizontalNamecard.HorizontalNamecard")))))))

(fn ConstructionScript
  (bind _namecard (Variables|Default|GetNamecard))
  (Utilities|FlowControl|Sequence
    (:then_0
      (Utilities|IsValid (Variables|Default|GetText3D)
        (:Is%20Valid
          (Variables|/Script/Text3D.Text3DComponent|SetText (Variables|Default|GetText3D) (Variables|InteractionControls|GetPersonName)))))
    (:then_1
      (Utilities|IsValid (Variables|Default|GetNamecard)
        (:Is%20Valid
          (switch Utilities|FlowControl|Switch|SwitchonE_NamecardType (Variables|InteractionControls|GetNamecardType)
            (:NewEnumerator0
              (Components|StaticMesh|SetStaticMesh _namecard "/Game/HungryGaussians/Assets/Models/Namecard/RoundedNamecard.RoundedNamecard"))
            (:NewEnumerator1
              (Components|StaticMesh|SetStaticMesh _namecard "/Game/HungryGaussians/Assets/Models/Namecard/VerticalNamecard.VerticalNamecard"))))))))

(fn GetLevelName)

(fn IsHovering
  (return false))