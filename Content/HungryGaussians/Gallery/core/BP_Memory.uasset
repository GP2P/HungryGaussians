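; BP_Memory is a gallery Blueprint that plays an audio file from disk when its PlayAudio event is called.
; PlayAudio creates a Runtime Audio Importer and imports the WAV at Content.FilePath, printing debug messages along the way.
; On a successful result, the imported sound wave plays as non-spatialized 2D audio at boosted volume.
; Nothing in this Blueprint calls PlayAudio, and failed imports are not handled.
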(event Custom|PlayAudio
  (bind _content (Variables|Default|GetContent))
  (bind _filepath (Utilities|Struct|BreakST_Memory _content))
  (Development|PrintString "audio triggered on cube")
  (bind _returnvalue (Class|RuntimeAudioImporterLibrary|CreateRuntimeAudioImporter))
  (bind _output_get (Variables|Default|SetAudioImporter _returnvalue))
  (EventDispatchers|BindEventtoOnResult _output_get (delegate Custom|OnResult_Event))
  (Class|RuntimeAudioImporterLibrary|ImportAudiofromFile (Variables|Default|GetAudioImporter) _filepath "Wav")
  (Development|PrintString _filepath))

(event Custom|OnResult_Event
  (params (Importer :type Runtime%20Audio%20Importer%20Library%20Object%20Reference) (ImportedSoundWave :type Imported%20Sound%20Wave%20Object%20Reference) (Status :type ERuntimeImportStatus%20Enum :default "SuccessfulImport"))
  (switch Utilities|FlowControl|Switch|SwitchonERuntimeImportStatus Status
    (:SuccessfulImport
      (Variables|Default|SetAudioImporter Importer)
      (Audio|SpawnSound2D ImportedSoundWave 3.0 1.0 0.0 0))))

(event EventBeginPlay)

(event Collision|EventActorBeginOverlap
  (params (OtherActor :type Actor%20Object%20Reference)))

(event EventTick
  (params (DeltaSeconds :type Float%20%28single-precision%29)))

(fn ConstructionScript)