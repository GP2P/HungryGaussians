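; BP_Person_Parent is a parent actor for people, with scaffolding for hover detection, turning toward the player and teleporting to a level.
; Construction caches the VRSpectator, whose view tracer supplies a hit result intended for hover state.
; RotateToPlayer interpolates yaw toward a pawn.
; Much is disconnected: overlap timers, tracing and level loading never run, teleport only prints debug text, and the level and hover getters return placeholders.
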(event OnComponentBeginOverlap(SphereLookAtPlayer)
  (params (OverlappedComponent :type Primitive%20Component%20Object%20Reference) (OtherActor :type Actor%20Object%20Reference) (OtherComp :type Primitive%20Component%20Object%20Reference) (OtherBodyIndex :type Integer) (bFromSweep :type Boolean) (SweepResult :type Hit%20Result%20Structure%20%28by%20ref%29))
  ;[1 0 0.04687] (Not 100% working) (Overlap to have actor face player
)

(event OnComponentEndOverlap(SphereLookAtPlayer)
  (params (OverlappedComponent :type Primitive%20Component%20Object%20Reference) (OtherActor :type Actor%20Object%20Reference) (OtherComp :type Primitive%20Component%20Object%20Reference) (OtherBodyIndex :type Integer))
  ;[1 0 0.04687] (Not 100% working) (Overlap to have actor face player
)

(event Custom|RotateToPlayer
  ;[1 0 0.04687] (Not 100% working) (Overlap to have actor face player
  (Transformation|SetActorRotation (Math|Rotator|MakeRotator 0.0 0.0 (.yaw (Math|Interpolation|RInterpTo (Transformation|GetActorRotation) (Math|Rotator|FindLookatRotation (Transformation|GetActorLocation) (Transformation|GetActorLocation (stale _aspawn))) (Utilities|Time|GetWorldDeltaSeconds) 1.0)))))

(event EventBeginPlay)

(event EventOnBeginHoverOverActor
  (Development|PrintString "On Hover Begin"))

(event EventOnEndHoverOverActor)

(event EventTick
  (params (DeltaSeconds :type Float%20%28single-precision%29)))

(event EventSetIsHovering
  (params (bHovering :type Boolean))
  (if bHovering
    (CallFunction|OnBeginHoverOverActor)
    (else
      (CallFunction|OnEndHoverOverActor))))

(event EventTeleporttoLevel
  (Development|PrintString "fuck"))

(fn ConstructionScript
  (bind _returnvalue (Actor|GetActorOfClass "/Game/VRSpectator/VRSpectator.VRSpectator_C"))
  (Utilities|IsValid _returnvalue
    (:Is%20Valid
      (Variables|InteractableControls|SetPlayer _returnvalue))))

(fn MakeViewTracer
  (bind _bhit (Default|MakeViewTracer (Variables|InteractableControls|GetPlayer) "Persistent"))
  (return _bhit))

(fn GetLevelName
  (return "None"))

(fn IsHovering
  (return false))